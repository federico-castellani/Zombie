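; Purchasable Stamina Up perk station that the player buys with points.
; An overlap box shows or hides an interact widget with the cost while the player lacks the perk.
; OnInteract checks points on the soldier's BPCStats component, deducts the cost, adds the perk, removes the prompt and plays a drink montage.
; The widget and soldier reference are cached on BeginPlay.
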(event OnComponentBeginOverlap(Box)
  (params (OverlappedComponent :type Primitive%20Component%20Object%20Reference) (OtherActor :type Actor%20Object%20Reference) (OtherComp :type Primitive%20Component%20Object%20Reference) (OtherBodyIndex :type Integer) (bFromSweep :type Boolean) (SweepResult :type Hit%20Result%20Structure%20%28by%20ref%29))
  (if (== OtherActor (Game|GetPlayerCharacter 0))
    (if (not (Variables|/Game/BLUEPRINTS/BPC_Stats.BPC_Stats_C|GetHasStaminaUp (Variables|/Game/BLUEPRINTS/BP_soldier.BP_soldier_C|GetBPC_Stats (Variables|Default|GetBP%20Soldier%20Ref))))
      (UserInterface|Viewport|AddtoViewport (Variables|Default|GetInteract%20Ref) 0)
      (Variables|/Script/UMG.TextBlock|SetText (Variables|/Game/WIDGET/WBP_Interact.WBP_Interact_C|GetPunti (Variables|Default|GetInteract%20Ref)) (Utilities|Text|ToText(Float) (Variables|Default|GetCosto) "HalfToEven"))
      (Variables|/Script/UMG.TextBlock|SetText (Variables|/Game/WIDGET/WBP_Interact.WBP_Interact_C|GetAzione (Variables|Default|GetInteract%20Ref)) "acquistare Stamina Up"))))

(event OnComponentEndOverlap(Box)
  (params (OverlappedComponent :type Primitive%20Component%20Object%20Reference) (OtherActor :type Actor%20Object%20Reference) (OtherComp :type Primitive%20Component%20Object%20Reference) (OtherBodyIndex :type Integer))
  (if (== OtherActor (Game|GetPlayerCharacter 0))
    (if (not (Variables|/Game/BLUEPRINTS/BPC_Stats.BPC_Stats_C|GetHasStaminaUp (Variables|/Game/BLUEPRINTS/BP_soldier.BP_soldier_C|GetBPC_Stats (Variables|Default|GetBP%20Soldier%20Ref))))
      (Widget|RemovefromParent (Variables|Default|GetInteract%20Ref)))))

(event EventBeginPlay
  (bind _returnvalue (UserInterface|CreateWidget "/Game/WIDGET/WBP_Interact.WBP_Interact_C"))
  (Variables|Default|SetInteract%20Ref _returnvalue)
  (bind _asbp_soldier (Utilities|Casting|CastToBP_soldier (Game|GetPlayerCharacter 0)))
  (Variables|Default|SetBP%20Soldier%20Ref _asbp_soldier))

(event EventOnInteract
  (bind _bp_soldier_ref (Variables|Default|GetBP%20Soldier%20Ref))
  (bind _bpc_stats (Variables|/Game/BLUEPRINTS/BP_soldier.BP_soldier_C|GetBPC_Stats _bp_soldier_ref))
  (if (not (Variables|/Game/BLUEPRINTS/BPC_Stats.BPC_Stats_C|GetHasStaminaUp _bpc_stats))
    (if (>= (Variables|/Game/BLUEPRINTS/BPC_Stats.BPC_Stats_C|GetPunti _bpc_stats) (Variables|Default|GetCosto))
      (Default|DecreasePoints (Variables|/Game/BLUEPRINTS/BP_soldier.BP_soldier_C|GetBPC_Stats (Variables|Default|GetBP%20Soldier%20Ref)) (Variables|Default|GetCosto))
      (Default|AddPerk (Variables|/Game/BLUEPRINTS/BP_soldier.BP_soldier_C|GetBPC_Stats (Variables|Default|GetBP%20Soldier%20Ref)) "NewEnumerator2")
      (Widget|RemovefromParent (Variables|Default|GetInteract%20Ref))
      (Animation|PlayAnimMontage (Variables|Default|GetBP%20Soldier%20Ref) "/Game/ANIMATIONS/Soldier/Drink_Perk.Drink_Perk" 1.0 "None"))))

(fn ConstructionScript)