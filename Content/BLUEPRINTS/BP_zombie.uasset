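; Zombie enemy character that climbs in on spawn, fights the player soldier and awards points when damaged or killed.
; After the climb montage it lifts its capsule, sets the AI blackboard's Spawned flag and picks one of two walk speeds at random.
; ZombieAttack plays a montage with a delayed distance check before damaging the player's stats component.
; Death disables collision, decrements the soldier's zombie count, occasionally drops a power-up and destroys the actor.
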(event Custom|Zombie%20Attack
  ;[0.05098 0.05098 0.05098] Attack
  (if (not (Variables|/Game/BLUEPRINTS/BPC_Stats.BPC_Stats_C|GetIsDead (Variables|/Game/BLUEPRINTS/BP_soldier.BP_soldier_C|GetBPC_Stats (Variables|Default|GetBP%20Soldier%20Ref))))
    (CallFunction|Damage)
    (Animation|PlayAnimMontage "/Game/ANIMATIONS/Zombi/Zombie_Attack_Montage.Zombie_Attack_Montage" 1.2 "None")))

(event Custom|Damage
  ;[0.05098 0.05098 0.05098] Attack
  (Utilities|FlowControl|Delay 1.0)
  (if (<= (Math|Vector|VectorLength (- (Transformation|GetActorLocation (Variables|Default|GetBP%20Soldier%20Ref)) (Transformation|GetActorLocation))) 1.2e+02)
    (Default|DecreaseHealth (Variables|/Game/BLUEPRINTS/BP_soldier.BP_soldier_C|GetBPC_Stats (Variables|Default|GetBP%20Soldier%20Ref)) 5e+01)))

(event Custom|Death
  (bind _returnvalue (Transformation|GetActorTransform))
  (bind (_location _rotation _scale) (Math|Transform|BreakTransform _returnvalue))
  ;[0.05098 0.05098 0.05098] Death
  (Collision|SetCollisionEnabled (Variables|Collision|GetCapsuleComponent) "NoCollision")
  (Animation|PlayAnimMontage "/Game/ANIMATIONS/Zombi/Zombie_Death_Montage.Zombie_Death_Montage" 1.0 "None")
  (Utilities|FlowControl|Delay 2.2)
  (Default|CustomDecrementZombies (Variables|Default|GetBP%20Soldier%20Ref))
  (if (Math|Random|RandomBoolwithWeight 0.1)
    (Game|SpawnActorfromClass "/Game/BLUEPRINTS/BP_PowerUp.BP_PowerUp_C" (Math|Transform|MakeTransform (- _location "0.000000,0.000000,100.000000") _rotation _scale) "AlwaysSpawn" "MultiplyWithRoot" 0 0))
  (Actor|DestroyActor))

(event EventBeginPlay
  ;[0.05098 0.05098 0.05098] Spawn
  (bind _asbp_soldier (Utilities|Casting|CastToBP_soldier (Game|GetPlayerCharacter 0)))
  (Variables|Default|SetBP%20Soldier%20Ref _asbp_soldier)
  (bind _returnvalue (Animation|PlayAnimMontage "/Game/ANIMATIONS/Zombi/Zombie_Climbing_Montage.Zombie_Climbing_Montage" 1.0 "None"))
  (Utilities|FlowControl|Delay _returnvalue)
  (Class|SceneComponent|AddLocalTransform (Variables|Collision|GetCapsuleComponent) (Math|Transform|MakeTransform (+ "" "0.000000,0.000000,270.000000")) false false)
  (AI|Components|Blackboard|SetValueasBool (AI|GetBlackboard (AI|GetAIController self)) (Utilities|Name|MakeLiteralName "Spawned") true)
  (if (Math|Random|RandomBool)
    (Variables|/Script/Engine.CharacterMovementComponent|SetMaxWalkSpeed (Variables|Character|GetCharacterMovement) 5e+02)
    (else
      (Variables|/Script/Engine.CharacterMovementComponent|SetMaxWalkSpeed (Variables|Character|GetCharacterMovement) 3e+02))))

(event Game|Damage|EventAnyDamage
  (params (Damage :type Float%20%28single-precision%29) (DamageType :type Damage%20Type%20Object%20Reference) (InstigatedBy :type Controller%20Object%20Reference) (DamageCauser :type Actor%20Object%20Reference))
  ;[0.05098 0.05098 0.05098] Damage
  (Default|DecreaseHealth (Variables|Default|GetBPC_Zombie_Stats) Damage)
  (if (Variables|/Game/BLUEPRINTS/BPC_Zombie_Stats.BPC_Zombie_Stats_C|GetIsDead (Variables|Default|GetBPC_Zombie_Stats))
    (Default|AddPoints (Variables|/Game/BLUEPRINTS/BP_soldier.BP_soldier_C|GetBPC_Stats (Variables|Default|GetBP%20Soldier%20Ref)) 5e+01)
    (CallFunction|Death)
    (else
      (Default|AddPoints (Variables|/Game/BLUEPRINTS/BP_soldier.BP_soldier_C|GetBPC_Stats (Variables|Default|GetBP%20Soldier%20Ref)) 1e+01))))

(fn ConstructionScript)