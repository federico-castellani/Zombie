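; BP_Gate is a gate Blueprint that shows an interaction prompt when the player is near.
; On BeginPlay it creates a WBP_Interact widget once and keeps a reference to it.
; The MessageBox component's overlap events add that widget to the viewport when player character 0 enters and remove it on exit.
; The graph contains only the prompt logic, with no input handling or gate movement.
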(event OnComponentBeginOverlap(MessageBox)
  (params (OverlappedComponent :type Primitive%20Component%20Object%20Reference) (OtherActor :type Actor%20Object%20Reference) (OtherComp :type Primitive%20Component%20Object%20Reference) (OtherBodyIndex :type Integer) (bFromSweep :type Boolean) (SweepResult :type Hit%20Result%20Structure%20%28by%20ref%29))
  (if (== OtherActor (Game|GetPlayerCharacter 0))
    (UserInterface|Viewport|AddtoViewport (Variables|Default|GetInteract%20Ref) 0)))

(event OnComponentEndOverlap(MessageBox)
  (params (OverlappedComponent :type Primitive%20Component%20Object%20Reference) (OtherActor :type Actor%20Object%20Reference) (OtherComp :type Primitive%20Component%20Object%20Reference) (OtherBodyIndex :type Integer))
  (if (== OtherActor (Game|GetPlayerCharacter 0))
    (Widget|RemovefromParent (Variables|Default|GetInteract%20Ref))))

(event EventBeginPlay
  (bind _returnvalue (UserInterface|CreateWidget "/Game/WIDGET/WBP_Interact.WBP_Interact_C"))
  (Variables|Default|SetInteract%20Ref _returnvalue))

(fn ConstructionScript)