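; Player controller that manages the start menu and in-game HUD.
; On BeginPlay it creates the start menu, switches to UI-only input, pauses the game and shows the cursor.
; A separate CreateHUD event adds the HUD, hands its reference to the soldier character's stats component, then restores game-only input, unpauses and hides the cursor.
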(event Custom|Create%20HUD
  (bind _returnvalue (Game|GetPlayerController 0))
  ;[0.05098 0.05098 0.05098] HUD
  (bind _returnvalue_2 (UserInterface|CreateWidget "/Game/WIDGET/WBP_HUD.WBP_HUD_C" _returnvalue))
  (bind _output_get (Variables|Default|SetHUD%20Ref _returnvalue_2))
  (UserInterface|Viewport|AddtoViewport _output_get 0)
  (bind _asbp_soldier (Utilities|Casting|CastToBP_soldier (Game|GetPlayerCharacter 0)))
  (Variables|/Game/BLUEPRINTS/BPC_Stats.BPC_Stats_C|SetHUD%20Ref (Variables|/Game/BLUEPRINTS/BP_soldier.BP_soldier_C|GetBPC_Stats _asbp_soldier) (Variables|Default|GetHUD%20Ref))
  (Input|SetInputModeGameOnly _returnvalue false)
  (Game|SetGamePaused false)
  (Variables|Default|SetbShowMouseCursor false))

(event Custom|Create%20StartMenu
  (bind _returnvalue (Game|GetPlayerController 0))
  ;[0.05098 0.05098 0.05098] StartMenu
  (bind _returnvalue_2 (UserInterface|CreateWidget "/Game/WIDGET/WBP_StartMenu.WBP_StartMenu_C" _returnvalue))
  (bind _output_get (Variables|Default|SetStartMenu%20Ref _returnvalue_2))
  (UserInterface|Viewport|AddtoViewport _output_get 0)
  (Input|SetInputModeUIOnly _returnvalue 0 "DoNotLock" false)
  (Game|SetGamePaused true)
  (Variables|Default|SetbShowMouseCursor true))

(event EventBeginPlay
  (CallFunction|CreateStartMenu))

(fn ConstructionScript)