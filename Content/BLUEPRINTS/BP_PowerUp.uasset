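; BP_PowerUp is a short-lived zombie-mode pickup that grants one of four random bonuses to the player's BP_soldier.
; The construction script rolls the type and sets its matching mesh.
; Player overlap applies the effect, then destroys the actor: instant kill, refilled ammo for both weapons, a nuke killing every BP_zombie for points, or bonus points.
; Uncollected pickups destroy themselves after a brief delay from BeginPlay.
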(event EventBeginPlay
  (bind _asbp_soldier (Utilities|Casting|CastToBP_soldier (Game|GetPlayerCharacter 0)))
  (Variables|Default|SetBP%20Soldier%20Ref _asbp_soldier)
  (Utilities|FlowControl|Delay 6.0)
  (Actor|DestroyActor))

(event Collision|EventActorBeginOverlap
  (params (OtherActor :type Actor%20Object%20Reference))
  (bind _bp_soldier_ref (Variables|Default|GetBP%20Soldier%20Ref))
  (bind _bp_soldier_ref_2 (Variables|Default|GetBP%20Soldier%20Ref))
  (bind _bpc_stats (Variables|/Game/BLUEPRINTS/BP_soldier.BP_soldier_C|GetBPC_Stats _bp_soldier_ref))
  (if (== OtherActor (Game|GetPlayerCharacter 0))
    (switch Utilities|FlowControl|Switch|SwitchonEnum_PowerUps (Variables|Default|GetPowerUp%20Type)
      (:NewEnumerator0
        ;[0.05098 0.05098 0.05098] Instant Kill
        (Default|ActivateInstantKill (Variables|Default|GetBP%20Soldier%20Ref)))
      (:NewEnumerator1
        ;[0.05098 0.05098 0.05098] Max Ammo
        (Variables|/Game/BLUEPRINTS/BP_soldier.BP_soldier_C|SetActiveWeapon _bp_soldier_ref_2 (Utilities|Struct|MakeStruct_Weapons (.nome (Variables|/Game/BLUEPRINTS/BP_soldier.BP_soldier_C|GetActiveWeapon _bp_soldier_ref_2)) (.damage (Variables|/Game/BLUEPRINTS/BP_soldier.BP_soldier_C|GetActiveWeapon _bp_soldier_ref_2)) (.firerate (Variables|/Game/BLUEPRINTS/BP_soldier.BP_soldier_C|GetActiveWeapon _bp_soldier_ref_2)) (.skeletalmesh (Variables|/Game/BLUEPRINTS/BP_soldier.BP_soldier_C|GetActiveWeapon _bp_soldier_ref_2)) (.weapontype (Variables|/Game/BLUEPRINTS/BP_soldier.BP_soldier_C|GetActiveWeapon _bp_soldier_ref_2)) (.magazinesize (Variables|/Game/BLUEPRINTS/BP_soldier.BP_soldier_C|GetActiveWeapon _bp_soldier_ref_2)) (.ammomagazinesize (Variables|/Game/BLUEPRINTS/BP_soldier.BP_soldier_C|GetActiveWeapon _bp_soldier_ref_2)) (.magazinesize (Variables|/Game/BLUEPRINTS/BP_soldier.BP_soldier_C|GetActiveWeapon _bp_soldier_ref_2)) (.ammomagazinesize (Variables|/Game/BLUEPRINTS/BP_soldier.BP_soldier_C|GetActiveWeapon _bp_soldier_ref_2)) "0.000000,0.000000,0.000000"))
        (Variables|/Game/BLUEPRINTS/BP_soldier.BP_soldier_C|SetSecondWeapon _bp_soldier_ref_2 (Utilities|Struct|MakeStruct_Weapons (.nome (Variables|/Game/BLUEPRINTS/BP_soldier.BP_soldier_C|GetSecondWeapon _bp_soldier_ref_2)) (.damage (Variables|/Game/BLUEPRINTS/BP_soldier.BP_soldier_C|GetSecondWeapon _bp_soldier_ref_2)) (.firerate (Variables|/Game/BLUEPRINTS/BP_soldier.BP_soldier_C|GetSecondWeapon _bp_soldier_ref_2)) (.skeletalmesh (Variables|/Game/BLUEPRINTS/BP_soldier.BP_soldier_C|GetSecondWeapon _bp_soldier_ref_2)) (.weapontype (Variables|/Game/BLUEPRINTS/BP_soldier.BP_soldier_C|GetSecondWeapon _bp_soldier_ref_2)) (.magazinesize (Variables|/Game/BLUEPRINTS/BP_soldier.BP_soldier_C|GetSecondWeapon _bp_soldier_ref_2)) (.ammomagazinesize (Variables|/Game/BLUEPRINTS/BP_soldier.BP_soldier_C|GetSecondWeapon _bp_soldier_ref_2)) (.magazinesize (Variables|/Game/BLUEPRINTS/BP_soldier.BP_soldier_C|GetSecondWeapon _bp_soldier_ref_2)) (.ammomagazinesize (Variables|/Game/BLUEPRINTS/BP_soldier.BP_soldier_C|GetSecondWeapon _bp_soldier_ref_2)) "0.000000,0.000000,0.000000"))
        (Default|ChangeAmmo _bpc_stats (.ammo (Variables|/Game/BLUEPRINTS/BP_soldier.BP_soldier_C|GetActiveWeapon _bp_soldier_ref)))
        (Default|ChangeAmmoMagazine _bpc_stats (.ammomagazine (Variables|/Game/BLUEPRINTS/BP_soldier.BP_soldier_C|GetActiveWeapon _bp_soldier_ref))))
      (:NewEnumerator2
        ;[0.05098 0.05098 0.05098] Nuke
        (bind _outactors (Actor|GetAllActorsOfClass "/Game/BLUEPRINTS/BP_zombie.BP_zombie_C"))
        (for _array_element _outactors
          (Default|Death _array_element))
        (Default|AddPoints (Variables|/Game/BLUEPRINTS/BP_soldier.BP_soldier_C|GetBPC_Stats (Variables|Default|GetBP%20Soldier%20Ref)) 4e+02))
      (:NewEnumerator3
        ;[0.05098 0.05098 0.05098] Bonus Points
        (Default|AddPoints (Variables|/Game/BLUEPRINTS/BP_soldier.BP_soldier_C|GetBPC_Stats (Variables|Default|GetBP%20Soldier%20Ref)) 1.5e+03)))
    (Actor|DestroyActor)))

(fn ConstructionScript
  (switch int (Math|Random|RandomIntegerinRange 0 3)
    (:0
      ;[0.05098 0.05098 0.05098] Instant Kill
      (Components|StaticMesh|SetStaticMesh (Variables|Default|GetInstant%20Kill) "/Game/Megascans/3D_Assets/PowerUps/skull.skull")
      (Variables|Default|SetPowerUp%20Type "NewEnumerator0"))
    (:1
      ;[0.05098 0.05098 0.05098] Max Ammo
      (Components|StaticMesh|SetStaticMesh (Variables|Default|GetMax%20Ammo) "/Game/Megascans/3D_Assets/PowerUps/ammo.ammo")
      (Variables|Default|SetPowerUp%20Type "NewEnumerator1"))
    (:2
      ;[0.05098 0.05098 0.05098] Nuke
      (Components|StaticMesh|SetStaticMesh (Variables|Default|GetNuke) "/Game/Megascans/3D_Assets/PowerUps/nuke.nuke")
      (Variables|Default|SetPowerUp%20Type "NewEnumerator2"))
    (:3
      ;[0.05098 0.05098 0.05098] Bonus Points
      (Components|StaticMesh|SetStaticMesh (Variables|Default|GetBonus%20Points) "/Game/Megascans/3D_Assets/PowerUps/bonus_points.bonus_points")
      (Variables|Default|SetPowerUp%20Type "NewEnumerator3"))))