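; BP_ZombieSpawner is a spawner actor that releases a batch of BP_zombie actors once activated.
; The AttivaSpawner event sets IsActive, after which Tick spawns one zombie per frame and decrements ZombiesToSpawn until none remain.
; Each zombie takes the spawner's transform lowered 200 units in Z and always spawns regardless of collision.
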(event Custom|Spawn%20Zombie
  (bind _returnvalue (Transformation|GetActorTransform))
  (bind (_location _rotation _scale) (Math|Transform|BreakTransform _returnvalue))
  (Game|SpawnActorfromClass "/Game/BLUEPRINTS/BP_zombie.BP_zombie_C" (Math|Transform|MakeTransform (+ _location "0.000000,0.000000,-200.000000") _rotation _scale) "AlwaysSpawn" "MultiplyWithRoot" 0 0))

(event Custom|AttivaSpawner
  (Variables|Default|SetIsActive true))

(event EventTick
  (params (DeltaSeconds :type Float%20%28single-precision%29))
  (if (Variables|Default|GetIsActive)
    (if (> (Variables|Default|GetZombiesToSpawn) 0)
      (CallFunction|SpawnZombie)
      (Math|Integer|DecrementInt (Variables|Default|GetZombiesToSpawn)))))

(fn ConstructionScript)