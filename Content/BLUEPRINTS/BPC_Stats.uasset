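; BPC_Stats is a stats component that tracks health and a death flag, with functions for healing and damage.
; DecreaseHealth floors health at zero and sets IsDead there, while IncreaseHealth adds without a cap because its max-health comparison is left unconnected.
; Both functions call UpdateHealthBar, which pushes the health ratio and value to the HUD's bar and text through HUDRef.
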(event EventBeginPlay)

(event EventTick
  (params (DeltaSeconds :type Float%20%28single-precision%29)))

(fn IncreaseHealth
  (params (Heal :type Float%20%28double-precision%29))
  (if true
    (Variables|Default|SetHealth (+ Heal (Variables|Default|GetHealth)))
    (else
      (Variables|Default|SetHealth (Variables|Default|GetMaxHealth))))
  (CallFunction|UpdateHealthBar))

(fn DecreaseHealth
  (params (Damage :type Float%20%28double-precision%29))
  (if (> (- (Variables|Default|GetHealth) Damage) 0.0)
    (Variables|Default|SetHealth (- (Variables|Default|GetHealth) Damage))
    (else
      (Variables|Default|SetHealth 0.0)))
  (CallFunction|UpdateHealthBar)
  (if (== (Variables|Default|GetHealth) 0.0)
    (Variables|Default|SetIsDead true)))

(fn UpdateHealthBar
  (Progress|SetPercent (Variables|/Game/WIDGET/WBP_HUD.WBP_HUD_C|GetHealthBar (Variables|Default|GetHUD%20Ref)) (/ (Variables|Default|GetHealth) (Variables|Default|GetMaxHealth)))
  (Variables|/Script/UMG.TextBlock|SetText (Variables|/Game/WIDGET/WBP_HUD.WBP_HUD_C|GetHealth (Variables|Default|GetHUD%20Ref)) (Utilities|Text|ToText(Float) (Variables|Default|GetHealth) "HalfToEven")))