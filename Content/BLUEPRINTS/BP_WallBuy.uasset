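; BP_WallBuy is a wall weapon shop where the player spends points on a weapon or its ammo.
; The construction script loads the weapon from DT_Weapons by WeaponName and sets the displayed mesh.
; Box overlap compares skeletal meshes against BP_soldier's two weapon slots and shows WBP_Interact with the matching price.
; OnInteract checks points in BPCStats, then adds the weapon or refills the matching slot's ammo and deducts the cost.
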(event OnComponentBeginOverlap(Box)
  (params (OverlappedComponent :type Primitive%20Component%20Object%20Reference) (OtherActor :type Actor%20Object%20Reference) (OtherComp :type Primitive%20Component%20Object%20Reference) (OtherBodyIndex :type Integer) (bFromSweep :type Boolean) (SweepResult :type Hit%20Result%20Structure%20%28by%20ref%29))
  (bind _bp_soldier_ref (Variables|Default|GetBP%20Soldier%20Ref))
  (bind _weapon (Variables|Default|GetWeapon))
  (if (== OtherActor (Game|GetPlayerCharacter 0))
    (Variables|Default|SetCanInteract true)
    (bind _output_get (Variables|Default|SetNotHasWeapon (and (!= (.skeletalmesh (Variables|/Game/BLUEPRINTS/BP_soldier.BP_soldier_C|GetActiveWeapon _bp_soldier_ref)) (.skeletalmesh _weapon)) (!= (.skeletalmesh _weapon) (.skeletalmesh (Variables|/Game/BLUEPRINTS/BP_soldier.BP_soldier_C|GetSecondWeapon _bp_soldier_ref))))))
    (if _output_get
      ;[0.05098 0.05098 0.05098] Arma
      (UserInterface|Viewport|AddtoViewport (Variables|Default|GetInteract%20Ref) 0)
      (Variables|/Script/UMG.TextBlock|SetText (Variables|/Game/WIDGET/WBP_Interact.WBP_Interact_C|GetPunti (Variables|Default|GetInteract%20Ref)) (Utilities|Text|ToText(Float) (Variables|Default|GetCosto) "HalfToEven"))
      (Variables|/Script/UMG.TextBlock|SetText (Variables|/Game/WIDGET/WBP_Interact.WBP_Interact_C|GetAzione (Variables|Default|GetInteract%20Ref)) (Utilities|Text|ToText(String) (Utilities|String|Append (Utilities|String|MakeLiteralString "acquistare ") (.nome (Variables|Default|GetWeapon)))))
      (else
        ;[0.05098 0.05098 0.05098] Munizioni
        (UserInterface|Viewport|AddtoViewport (Variables|Default|GetInteract%20Ref) 0)
        (Variables|/Script/UMG.TextBlock|SetText (Variables|/Game/WIDGET/WBP_Interact.WBP_Interact_C|GetPunti (Variables|Default|GetInteract%20Ref)) (Utilities|Text|ToText(Float) (Variables|Default|GetCostoMunizioni) "HalfToEven"))
        (Variables|/Script/UMG.TextBlock|SetText (Variables|/Game/WIDGET/WBP_Interact.WBP_Interact_C|GetAzione (Variables|Default|GetInteract%20Ref)) (Utilities|Text|ToText(String) (Utilities|String|Append (Utilities|String|MakeLiteralString "acquistare le munizioni ") (.nome (Variables|Default|GetWeapon)))))))))

(event OnComponentEndOverlap(Box)
  (params (OverlappedComponent :type Primitive%20Component%20Object%20Reference) (OtherActor :type Actor%20Object%20Reference) (OtherComp :type Primitive%20Component%20Object%20Reference) (OtherBodyIndex :type Integer))
  (if (== OtherActor (Game|GetPlayerCharacter 0))
    (Widget|RemovefromParent (Variables|Default|GetInteract%20Ref))))

(event EventOnInteract
  (bind _bp_soldier_ref (Variables|Default|GetBP%20Soldier%20Ref))
  (bind _bpc_stats (Variables|/Game/BLUEPRINTS/BP_soldier.BP_soldier_C|GetBPC_Stats _bp_soldier_ref))
  (if (Variables|Default|GetCanInteract)
    (if (Variables|Default|GetNotHasWeapon)
      (if (>= (Variables|/Game/BLUEPRINTS/BPC_Stats.BPC_Stats_C|GetPunti (Variables|/Game/BLUEPRINTS/BP_soldier.BP_soldier_C|GetBPC_Stats (Variables|Default|GetBP%20Soldier%20Ref))) (Variables|Default|GetCosto))
        (Default|AddWeapon (Variables|Default|GetBP%20Soldier%20Ref) (Variables|Default|GetWeapon))
        (Default|DecreasePoints (Variables|/Game/BLUEPRINTS/BP_soldier.BP_soldier_C|GetBPC_Stats (Variables|Default|GetBP%20Soldier%20Ref)) (Variables|Default|GetCosto))
        (Widget|RemovefromParent (Variables|Default|GetInteract%20Ref))
        (Variables|Default|SetNotHasWeapon false))
      (elif (>= (Variables|/Game/BLUEPRINTS/BPC_Stats.BPC_Stats_C|GetPunti (Variables|/Game/BLUEPRINTS/BP_soldier.BP_soldier_C|GetBPC_Stats (Variables|Default|GetBP%20Soldier%20Ref))) (Variables|Default|GetCostoMunizioni))
        (if (== (.skeletalmesh (Variables|/Game/BLUEPRINTS/BP_soldier.BP_soldier_C|GetActiveWeapon (Variables|Default|GetBP%20Soldier%20Ref))) (.skeletalmesh (Variables|Default|GetWeapon)))
          (bind _output_get (Variables|/Game/BLUEPRINTS/BP_soldier.BP_soldier_C|SetActiveWeapon _bp_soldier_ref (Utilities|Struct|MakeStruct_Weapons (.nome (Variables|/Game/BLUEPRINTS/BP_soldier.BP_soldier_C|GetActiveWeapon _bp_soldier_ref)) (.damage (Variables|/Game/BLUEPRINTS/BP_soldier.BP_soldier_C|GetActiveWeapon _bp_soldier_ref)) (.firerate (Variables|/Game/BLUEPRINTS/BP_soldier.BP_soldier_C|GetActiveWeapon _bp_soldier_ref)) (.skeletalmesh (Variables|/Game/BLUEPRINTS/BP_soldier.BP_soldier_C|GetActiveWeapon _bp_soldier_ref)) (.weapontype (Variables|/Game/BLUEPRINTS/BP_soldier.BP_soldier_C|GetActiveWeapon _bp_soldier_ref)) (.magazinesize (Variables|/Game/BLUEPRINTS/BP_soldier.BP_soldier_C|GetActiveWeapon _bp_soldier_ref)) (.ammomagazinesize (Variables|/Game/BLUEPRINTS/BP_soldier.BP_soldier_C|GetActiveWeapon _bp_soldier_ref)) (.magazinesize (Variables|/Game/BLUEPRINTS/BP_soldier.BP_soldier_C|GetActiveWeapon _bp_soldier_ref)) (.ammomagazinesize (Variables|/Game/BLUEPRINTS/BP_soldier.BP_soldier_C|GetActiveWeapon _bp_soldier_ref)) "0.000000,0.000000,0.000000")))
          (Default|ChangeAmmo _bpc_stats (.magazinesize _output_get))
          (Default|ChangeAmmoMagazine _bpc_stats (.ammomagazinesize _output_get))
          (else
            (Variables|/Game/BLUEPRINTS/BP_soldier.BP_soldier_C|SetSecondWeapon _bp_soldier_ref (Utilities|Struct|MakeStruct_Weapons (.nome (Variables|/Game/BLUEPRINTS/BP_soldier.BP_soldier_C|GetSecondWeapon _bp_soldier_ref)) (.damage (Variables|/Game/BLUEPRINTS/BP_soldier.BP_soldier_C|GetSecondWeapon _bp_soldier_ref)) (.firerate (Variables|/Game/BLUEPRINTS/BP_soldier.BP_soldier_C|GetSecondWeapon _bp_soldier_ref)) (.skeletalmesh (Variables|/Game/BLUEPRINTS/BP_soldier.BP_soldier_C|GetSecondWeapon _bp_soldier_ref)) (.weapontype (Variables|/Game/BLUEPRINTS/BP_soldier.BP_soldier_C|GetSecondWeapon _bp_soldier_ref)) (.magazinesize (Variables|/Game/BLUEPRINTS/BP_soldier.BP_soldier_C|GetSecondWeapon _bp_soldier_ref)) (.ammomagazinesize (Variables|/Game/BLUEPRINTS/BP_soldier.BP_soldier_C|GetSecondWeapon _bp_soldier_ref)) (.magazinesize (Variables|/Game/BLUEPRINTS/BP_soldier.BP_soldier_C|GetSecondWeapon _bp_soldier_ref)) (.ammomagazinesize (Variables|/Game/BLUEPRINTS/BP_soldier.BP_soldier_C|GetSecondWeapon _bp_soldier_ref)) "0.000000,0.000000,0.000000"))))
        (Default|DecreasePoints (Variables|/Game/BLUEPRINTS/BP_soldier.BP_soldier_C|GetBPC_Stats (Variables|Default|GetBP%20Soldier%20Ref)) (Variables|Default|GetCostoMunizioni))
        (Variables|Default|SetCanInteract false)
        (Widget|RemovefromParent (Variables|Default|GetInteract%20Ref))))))

(event EventBeginPlay
  (bind _returnvalue (UserInterface|CreateWidget "/Game/WIDGET/WBP_Interact.WBP_Interact_C"))
  (Variables|Default|SetInteract%20Ref _returnvalue)
  (bind _asbp_soldier (Utilities|Casting|CastToBP_soldier (Game|GetPlayerCharacter 0)))
  (Variables|Default|SetBP%20Soldier%20Ref _asbp_soldier))

(fn ConstructionScript
  (bind _returnvalue (Utilities|GetDataTableRow "/Game/BLUEPRINTS/DT_Weapons.DT_Weapons" (Variables|Default|GetWeaponName))
    (:then
      (bind _output_get (Variables|Default|SetWeapon _returnvalue))
      (Components|SkeletalMesh|SetSkeletalMeshAsset (Variables|Default|GetArma) (.skeletalmesh _output_get)))))